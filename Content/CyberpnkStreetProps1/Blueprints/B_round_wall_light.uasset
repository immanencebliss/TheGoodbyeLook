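; Round wall light prop with an on/off toggle for its glow and spot light.
; The construction script creates a dynamic instance of M_round_wall_light on the WallLight component.
; When IsON is set, it applies the emission color and a clamped intensity and shows the SpotLight.
; Otherwise it applies the off intensity and hides the SpotLight; the event graph has no active logic.
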(fn `UserConstructionScript`
  (locals (EmissionOFF :type "Float (double-precision)"))
  (bind _wall_light (`self.wall_light`))
  (bind _spotlight (`self.SpotLight`))
  (if (`self.IsON`)
    (bind _returnvalue (`PrimitiveComponent.CreateDynamicMaterialInstance` _wall_light 0 "/Game/CyberpnkStreetProps1/Materials/M_round_wall_light.M_round_wall_light"))
    (`MaterialInstanceDynamic.SetScalarParameterValue` _returnvalue "EmissionIntensity" (`KismetMathLibrary.FClamp` (`self.EmissionIntensity`) 1.0 5000.0))
    (`MaterialInstanceDynamic.SetVectorParameterValue` _returnvalue "EmissionColor" (`self.EmissionColor`))
    (`SceneComponent.SetVisibility` _spotlight true false)
    (else
      (bind _returnvalue_2 (`PrimitiveComponent.CreateDynamicMaterialInstance` _wall_light 0 "/Game/CyberpnkStreetProps1/Materials/M_round_wall_light.M_round_wall_light"))
      (`MaterialInstanceDynamic.SetScalarParameterValue` _returnvalue_2 "EmissionIntensity" (`local.EmissionOFF`))
      (`SceneComponent.SetVisibility` _spotlight false false))))