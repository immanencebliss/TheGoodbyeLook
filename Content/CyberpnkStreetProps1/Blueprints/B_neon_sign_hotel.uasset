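; Blueprint for a neon hotel sign prop with a configurable lit or unlit look.
; The construction script creates a dynamic instance of the glass material on slot 1 of the sign mesh.
; The IsON flag switches the material parameter, applying emission color and intensity when lit or an off color when unlit.
; The event graph holds only disabled placeholder events, so the look does not change at runtime.
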(fn `UserConstructionScript`
  (bind _neon_sign_hotel (`self.neon_sign_hotel`))
  (if (`self.IsON`)
    (bind _returnvalue (`PrimitiveComponent.CreateDynamicMaterialInstance` _neon_sign_hotel 1 "/Game/CyberpnkStreetProps1/Materials/M_neon_sign_hotel_glass.M_neon_sign_hotel_glass"))
    (`MaterialInstanceDynamic.SetScalarParameterValue` _returnvalue "IsON" 1.0)
    (`MaterialInstanceDynamic.SetVectorParameterValue` _returnvalue "EmissionColor" (`self.EmissionColor`))
    (`MaterialInstanceDynamic.SetScalarParameterValue` _returnvalue "EmissionIntensity" (`self.EmissionIntensity`))
    (else
      (bind _returnvalue_2 (`PrimitiveComponent.CreateDynamicMaterialInstance` _neon_sign_hotel 1 "/Game/CyberpnkStreetProps1/Materials/M_neon_sign_hotel_glass.M_neon_sign_hotel_glass"))
      (`MaterialInstanceDynamic.SetScalarParameterValue` _returnvalue_2 "IsON" 0.0)
      (`MaterialInstanceDynamic.SetVectorParameterValue` _returnvalue_2 "OffColor" (`self.OffColor`)))))