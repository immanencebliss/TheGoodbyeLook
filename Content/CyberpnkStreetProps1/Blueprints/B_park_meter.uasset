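; Parking meter prop with an emissive panel that switches between standby and active states.
; The construction script builds a dynamic material on the ParkMeter component from IsON and IsActive, setting symbol and panel emission color and intensity.
; Sphere overlap events toggle PanelActive without filtering for players.
; Each overlap creates a fresh instance from M_park_meter, so construction-time parameters are not reapplied, and IsActive is untouched.
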(event `self.Sphere.OnComponentBeginOverlap`
  (params (OverlappedComponent :type "PrimitiveComponent Object Reference") (OtherActor :type "Actor Object Reference") (OtherComp :type "PrimitiveComponent Object Reference") (OtherBodyIndex :type Integer) (bFromSweep :type Boolean) (SweepResult :type "HitResult Structure (by ref)"))
  ;[1 1 1] this allows the parking meter panel to go from standby to active when a player enters the collision sphere (it might be applied also to the kiosk)
  (bind _returnvalue (`PrimitiveComponent.CreateDynamicMaterialInstance` (`self.park_meter`) 0 "/Game/CyberpnkStreetProps1/Materials/M_park_meter.M_park_meter"))
  (`MaterialInstanceDynamic.SetScalarParameterValue` _returnvalue "PanelActive" 1.0))

(event `self.Sphere.OnComponentEndOverlap`
  (params (OverlappedComponent :type "PrimitiveComponent Object Reference") (OtherActor :type "Actor Object Reference") (OtherComp :type "PrimitiveComponent Object Reference") (OtherBodyIndex :type Integer))
  ;[1 1 1] this allows the parking meter panel to go from standby to active when a player enters the collision sphere (it might be applied also to the kiosk)
  (bind _returnvalue (`PrimitiveComponent.CreateDynamicMaterialInstance` (`self.park_meter`) 0 "/Game/CyberpnkStreetProps1/Materials/M_park_meter.M_park_meter"))
  (`MaterialInstanceDynamic.SetScalarParameterValue` _returnvalue "PanelActive" 0.0))

(fn `UserConstructionScript`
  (bind _park_meter (`self.park_meter`))
  (if (`self.IsON`)
    (bind _returnvalue (`PrimitiveComponent.CreateDynamicMaterialInstance` _park_meter 0 "/Game/CyberpnkStreetProps1/Materials/M_park_meter.M_park_meter"))
    (`MaterialInstanceDynamic.SetScalarParameterValue` _returnvalue "SymbolON_EmissionIntensity" (`self.SymbolON_EmissionIntensity`))
    (`MaterialInstanceDynamic.SetVectorParameterValue` _returnvalue "SymbolON_EmissionColor" (`self.SymbolON_EmissionColor`))
    (`MaterialInstanceDynamic.SetScalarParameterValue` _returnvalue "IsON" 1.0)
    (if (`self.IsActive`)
      (`MaterialInstanceDynamic.SetScalarParameterValue` _returnvalue "IsActive" 1.0)
      (`MaterialInstanceDynamic.SetScalarParameterValue` _returnvalue "PanelActive_EmissionIntensity" (`self.PanelActive_EmissionIntensity`))
      (`MaterialInstanceDynamic.SetVectorParameterValue` _returnvalue "PanelActive_EmissionColor" (`self.PanelActive_EmissionColor`))
      (else
        (`MaterialInstanceDynamic.SetScalarParameterValue` _returnvalue "IsActive" 0.0)
        (`MaterialInstanceDynamic.SetScalarParameterValue` _returnvalue "PanelStandby_EmissionIntensity" (`self.PanelStandby_EmissionIntensity`))
        (`MaterialInstanceDynamic.SetVectorParameterValue` _returnvalue "PanelStandby_EmissionColor" (`self.PanelStandby_EmissionColor`))))
    (else
      (bind _returnvalue_2 (`PrimitiveComponent.CreateDynamicMaterialInstance` _park_meter 0 "/Game/CyberpnkStreetProps1/Materials/M_park_meter.M_park_meter"))
      (`MaterialInstanceDynamic.SetScalarParameterValue` _returnvalue_2 "IsON" 0.0))))