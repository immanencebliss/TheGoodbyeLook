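; Info kiosk street prop Blueprint whose emissive look is configured through exposed variables.
; The Construction Script creates a dynamic instance of M_info_kiosk on the InfoKiosk component and sets scalar and color parameters from those variables.
; IsON switches between a lit symbol and an off color, and when on, IsActive picks active or standby panel emission.
; The event graph has no runtime logic.
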(fn `UserConstructionScript`
  (bind _info_kiosk (`self.info_kiosk`))
  (if (`self.IsON`)
    (bind _returnvalue (`PrimitiveComponent.CreateDynamicMaterialInstance` _info_kiosk 0 "/Game/CyberpnkStreetProps1/Materials/M_info_kiosk.M_info_kiosk"))
    (`MaterialInstanceDynamic.SetScalarParameterValue` _returnvalue "SymbolON_EmissionIntensity" (`self.SymbolON_EmissionIntensity`))
    (`MaterialInstanceDynamic.SetVectorParameterValue` _returnvalue "SymbolON_EmissionColor" (`self.SymbolON_EmissionColor`))
    (`MaterialInstanceDynamic.SetScalarParameterValue` _returnvalue "IsON" 1.0)
    (if (`self.IsActive`)
      (`MaterialInstanceDynamic.SetScalarParameterValue` _returnvalue "IsActive" 1.0)
      (`MaterialInstanceDynamic.SetScalarParameterValue` _returnvalue "PanelActive_EmissionIntensity" (`self.PanelActive_EmissionIntensity`))
      (`MaterialInstanceDynamic.SetVectorParameterValue` _returnvalue "PanelActive_EmissionColor" (`self.PanelActive_EmissionColor`))
      (else
        (`MaterialInstanceDynamic.SetScalarParameterValue` _returnvalue "IsActive" 0.0)
        (`MaterialInstanceDynamic.SetScalarParameterValue` _returnvalue "PanelStandby_EmissionIntensity" (`self.PanelStandby_EmissionIntensity`))
        (`MaterialInstanceDynamic.SetVectorParameterValue` _returnvalue "PanelStandby_EmissionColor" (`self.PanelStandby_EmissionColor`))))
    (else
      (bind _returnvalue_2 (`PrimitiveComponent.CreateDynamicMaterialInstance` _info_kiosk 0 "/Game/CyberpnkStreetProps1/Materials/M_info_kiosk.M_info_kiosk"))
      (`MaterialInstanceDynamic.SetScalarParameterValue` _returnvalue_2 "IsON" 0.0)
      (`MaterialInstanceDynamic.SetVectorParameterValue` _returnvalue_2 "SymbolOFFColor" (`self.SymbolOFF_Color`)))))