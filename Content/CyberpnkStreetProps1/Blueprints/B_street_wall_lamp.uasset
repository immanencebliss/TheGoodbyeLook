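; Street wall lamp prop Blueprint with an on/off switch, configured entirely in the Construction Script; the event graph has no active logic.
; It creates a dynamic instance of the lamp material on the mesh.
; When IsON is set, it applies a clamped emission intensity and a color and shows the SpotLight.
; Otherwise it applies the off-state intensity and hides the light.
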(fn `UserConstructionScript`
  (locals (EmissionIntOFF :type "Float (double-precision)" :default 0.0))
  (bind _street_wall_lamp (`self.street_wall_lamp`))
  (bind _spotlight (`self.SpotLight`))
  (if (`self.IsON`)
    (bind _returnvalue (`PrimitiveComponent.CreateDynamicMaterialInstance` _street_wall_lamp 0 "/Game/CyberpnkStreetProps1/Materials/M_street_wall_lamp.M_street_wall_lamp"))
    (`MaterialInstanceDynamic.SetScalarParameterValue` _returnvalue "EmissionIntensity" (`KismetMathLibrary.FClamp` (`self.EmissionIntensity`) 1.0 5000.0))
    (`MaterialInstanceDynamic.SetVectorParameterValue` _returnvalue "EmissionColor" (`self.EmissionColor`))
    (`SceneComponent.SetVisibility` _spotlight true false)
    (else
      (bind _returnvalue_2 (`PrimitiveComponent.CreateDynamicMaterialInstance` _street_wall_lamp 0 "/Game/CyberpnkStreetProps1/Materials/M_street_wall_lamp.M_street_wall_lamp"))
      (`MaterialInstanceDynamic.SetScalarParameterValue` _returnvalue_2 "EmissionIntensity" (`local.EmissionIntOFF`))
      (`SceneComponent.SetVisibility` _spotlight false false))))