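; Rising bollard street prop that builds a configurable row of bollards, each with a base and a pillar, in its construction script.
; Dynamic materials apply EmissionColor to the single pillar and the instanced pillars, and Height sets their Z position.
; Instances are cleared, then a countdown loop adds base and pillar instances along local X at DistanceBetween spacing for the bollards beyond the first.
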(fn `UserConstructionScript`
  (locals (numbertomake :type Integer) (current :type "Float (double-precision)") (distance :type "Float (double-precision)"))
  (bind _rising_bollard_baseinst (`self.rising_bollard_baseInst`))
  (bind _rising_bollard_pillarinst (`self.rising_bollard_pillarInst`))
  (bind _returnvalue (`PrimitiveComponent.CreateDynamicMaterialInstance` (`self.rising_bollard_pillar`) 0 null))
  (`MaterialInstanceDynamic.SetVectorParameterValue` _returnvalue "EmissionColor" (`self.EmissionColor`))
  (bind _returnvalue_2 (`PrimitiveComponent.CreateDynamicMaterialInstance` (`self.rising_bollard_pillarInst`) 0 null))
  (`MaterialInstanceDynamic.SetVectorParameterValue` _returnvalue_2 "EmissionColor" (`self.EmissionColor`))
  (`SceneComponent.K2_SetRelativeLocation` (`self.rising_bollard_pillar`) (`KismetMathLibrary.MakeVector` 0.0 0.0 (`self.Height`)) false false)
  (`InstancedStaticMeshComponent.ClearInstances` _rising_bollard_baseinst)
  (`InstancedStaticMeshComponent.ClearInstances` _rising_bollard_pillarinst)
  (set `local.numbertomake` (- (`self.NumberOfBollards`) 1))
  (set `local.distance` (`self.DistanceBetween`))
  (if (> (`local.numbertomake`) 0) :!label _label
    (bind _output_get (set `local.current` (+ (`local.current`) (`local.distance`))))
    (`InstancedStaticMeshComponent.AddInstance` _rising_bollard_baseinst (`KismetMathLibrary.MakeTransform` (`KismetMathLibrary.MakeVector` _output_get) (struct) (1.0 1.0 1.0)))
    (`InstancedStaticMeshComponent.AddInstance` _rising_bollard_pillarinst (`KismetMathLibrary.MakeTransform` (`KismetMathLibrary.MakeVector` _output_get 0.0 (`self.Height`)) (struct) (1.0 1.0 1.0)))
    (`/Engine/EditorBlueprintResources/StandardMacros.DecrementInt` (`local.numbertomake`)
      (:`  `
        (goto _label)))))