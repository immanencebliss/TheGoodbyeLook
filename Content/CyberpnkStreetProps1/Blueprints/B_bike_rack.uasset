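; Construction-script prop Blueprint that builds a row of bike racks for level dressing.
; It clears its instanced static mesh, then loops to add one fewer instance than the rack count, stepping along local X by the set spacing.
; The event graph holds only disabled stub events, so the actor has no runtime logic.
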(fn `UserConstructionScript`
  (locals (distance :type "Float (double-precision)" :default 70.0) (current :type "Float (double-precision)") (numbertomake :type Integer))
  (bind _instancedstaticmesh (`self.InstancedStaticMesh`))
  (`InstancedStaticMeshComponent.ClearInstances` _instancedstaticmesh)
  (set `local.numbertomake` (- (`self.NumberOfRacks`) 1))
  (set `local.distance` (`self.DistanceBetween`))
  (if (> (`local.numbertomake`) 0) :!label _label
    (bind _output_get (set `local.current` (+ (`local.current`) (`local.distance`))))
    (`InstancedStaticMeshComponent.AddInstance` _instancedstaticmesh (`KismetMathLibrary.MakeTransform` (`KismetMathLibrary.MakeVector` _output_get) (struct) (1.0 1.0 1.0)))
    (`/Engine/EditorBlueprintResources/StandardMacros.DecrementInt` (`local.numbertomake`)
      (:`  `
        (goto _label)))))