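; Prop Blueprint for a street sign post that shows either a bus or a metro sign on its glass.
; The construction script switches on Type to put the matching bus or metro glass material on slot 1 of the Post mesh.
; It then creates a dynamic material instance and sets its IsON scalar from the IsON flag to toggle the sign.
; The event graph holds no active logic.
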(fn `UserConstructionScript`
  (bind _post (`self.post`))
  (bind _ison (`self.IsON`))
  (switch `int` (`self.Type`)
    (:`0`
      (`PrimitiveComponent.SetMaterial` _post 1 "/Game/CyberpnkStreetProps1/Materials/M_sign_post_metro_bus_glass_BUS.M_sign_post_metro_bus_glass_BUS")
      (if _ison
        (bind _returnvalue (`PrimitiveComponent.CreateDynamicMaterialInstance` _post 1 "/Game/CyberpnkStreetProps1/Materials/M_sign_post_metro_bus_glass_BUS.M_sign_post_metro_bus_glass_BUS"))
        (`MaterialInstanceDynamic.SetScalarParameterValue` _returnvalue "IsON" 1.0)
        (else
          (bind _returnvalue_2 (`PrimitiveComponent.CreateDynamicMaterialInstance` _post 1 "/Game/CyberpnkStreetProps1/Materials/M_sign_post_metro_bus_glass_BUS.M_sign_post_metro_bus_glass_BUS"))
          (`MaterialInstanceDynamic.SetScalarParameterValue` _returnvalue_2 "IsON" 0.0))))
    (:`1`
      (`PrimitiveComponent.SetMaterial` _post 1 "/Game/CyberpnkStreetProps1/Materials/M_sign_post_metro_bus_glass_METRO.M_sign_post_metro_bus_glass_METRO")
      (if _ison
        (bind _returnvalue_3 (`PrimitiveComponent.CreateDynamicMaterialInstance` _post 1 "/Game/CyberpnkStreetProps1/Materials/M_sign_post_metro_bus_glass_METRO.M_sign_post_metro_bus_glass_METRO"))
        (`MaterialInstanceDynamic.SetScalarParameterValue` _returnvalue_3 "IsON" 1.0)
        (else
          (bind _returnvalue_4 (`PrimitiveComponent.CreateDynamicMaterialInstance` _post 1 "/Game/CyberpnkStreetProps1/Materials/M_sign_post_metro_bus_glass_METRO.M_sign_post_metro_bus_glass_METRO"))
          (`MaterialInstanceDynamic.SetScalarParameterValue` _returnvalue_4 "IsON" 0.0))))))