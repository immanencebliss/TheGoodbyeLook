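; Tall street lamp post prop whose lit or unlit state is set by an IsON flag.
; The construction script creates a dynamic material instance on the lamp mesh to drive its on/off switch, plus emission intensity and color when lit.
; It also shows or hides the spot light to match.
; The event graph has no active logic, so the state is only applied at construction.
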(fn `UserConstructionScript`
  (bind _lamppost_tall (`self.lamppost_tall`))
  (if (`self.IsON`)
    (bind _returnvalue (`PrimitiveComponent.CreateDynamicMaterialInstance` _lamppost_tall 0 "/Game/CyberpnkStreetProps1/Materials/M_lamp_post_tall.M_lamp_post_tall"))
    (`MaterialInstanceDynamic.SetScalarParameterValue` _returnvalue "EmissionIntensity" (`self.EmissionIntensity`))
    (`MaterialInstanceDynamic.SetVectorParameterValue` _returnvalue "EmissionColor" (`self.EmissionColor`))
    (`MaterialInstanceDynamic.SetScalarParameterValue` _returnvalue "IsON" 1.0)
    (`SceneComponent.SetVisibility` (`self.SpotLight`) true false)
    (else
      (bind _returnvalue_2 (`PrimitiveComponent.CreateDynamicMaterialInstance` _lamppost_tall 0 "/Game/CyberpnkStreetProps1/Materials/M_lamp_post_tall.M_lamp_post_tall"))
      (`MaterialInstanceDynamic.SetScalarParameterValue` _returnvalue_2 "IsON" 0.0)
      (`SceneComponent.SetVisibility` (`self.SpotLight`) false false))))