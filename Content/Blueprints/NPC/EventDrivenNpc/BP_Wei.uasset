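; Wei, a story NPC who talks with the player through the dialogue system and performs scripted boost and flee sequences.
; A dialogue event triggers the boost: Wei walks to a marker, plays a lift montage, enables climb-box collision and pauses until GiveBoost resumes it.
; Flee events, with no caller here, chain AI moves, timeline turns toward the player and gesture montages.
; Dialogue condition and value functions are mostly stubs.
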(event `Prepare Flee`
  (set `CharacterMovementComponent.MaxWalkSpeed` 281.0 (`self.CharacterMovement`))
  (`|AIMoveTo` self (0.0 0.0 0.0) (`self.Flee Start`) 0.0 true))

(event `Flee`
  (bind _mesh (`self.Mesh`))
  (bind (_lookstart_roll _lookstart_pitch) (`KismetMathLibrary.BreakRotator` (`self.LookStart`)))
  (bind (_returnvalue_roll _returnvalue_pitch _returnvalue_yaw) (`KismetMathLibrary.BreakRotator` (`KismetMathLibrary.FindLookAtRotation` (`self.K2_GetActorLocation`) (`self.K2_GetActorLocation` (`GameplayStatics.GetPlayerCharacter` 0)))))
  (set `self.LookStart` (`self.K2_GetActorRotation`))
  (bind (_direction _alpha) (`Timeline|Timeline_2`)
    (:`Update`
      (`self.K2_SetActorRotation` (`KismetMathLibrary.RLerp` (`self.LookStart`) (`KismetMathLibrary.MakeRotator` _lookstart_roll _lookstart_pitch _returnvalue_yaw) _alpha true)))
    (:`Finished`
      (`|PlayMontage` _mesh "/Game/Waving_Montage.Waving_Montage"
        (:`then`
          (`KismetSystemLibrary.Delay` 1.5)
          (`|PlayMontage` _mesh "/Game/Pointing_Montage.Pointing_Montage"
            (:`then`
              (`KismetSystemLibrary.Delay` 1.2)
              (`AnimInstance.Montage_Stop` (`SkeletalMeshComponent.GetAnimInstance` (`self.Mesh`)) 0.2 "/Game/Pointing_Montage.Pointing_Montage")
              (`|AIMoveTo` self (0.0 0.0 0.0) (`self.Flee End`)))))))))

(event `TriggerBoost`
  (`|AIMoveTo` self (0.0 0.0 0.0) (`self.BoostLocation`) 0.0 true
    (:`OnSuccess`
      (bind (_direction _alpha) (`Timeline|Timeline_0`)
        (:`Update`
          (`self.K2_SetActorRotation` (`KismetMathLibrary.RLerp` (`self.K2_GetActorRotation`) (`self.K2_GetActorRotation` (`self.BoostLocation`)) _alpha)))
        (:`Finished`
          (`self.OfferBoost`))))))

(event `OfferBoost`
  (`|PlayMontage` (`self.Mesh`) (`self.LiftMontage`)
    (:`then`
      (`KismetSystemLibrary.Delay` 2.0)
      (`PrimitiveComponent.SetCollisionEnabled` (`/Game/ClimbBox.Box` (`self.Climbbox1`)) "QueryAndPhysics")
      (`PrimitiveComponent.SetCollisionEnabled` (`/Game/ClimbBox.Box` (`self.Climbbox2`)) "QueryAndPhysics")
      (`KismetSystemLibrary.Delay` 4.0)
      (`AnimInstance.Montage_Pause` (`SkeletalMeshComponent.GetAnimInstance` (`self.Mesh`)) (`self.LiftMontage`)))))

(event `GiveBoost`
  (bind (_returnvalue_roll _returnvalue_pitch) (`KismetMathLibrary.BreakRotator` (`self.K2_GetActorRotation`)))
  (bind (_returnvalue_roll_2 _returnvalue_pitch_2 _returnvalue_yaw) (`KismetMathLibrary.BreakRotator` (`KismetMathLibrary.FindLookAtRotation` (`self.K2_GetActorLocation`) (`self.K2_GetActorLocation` (`GameplayStatics.GetPlayerCharacter` 0)))))
  (`|PlayMontage` (`self.Mesh`) (`self.LiftMontage`) 1.0 7.5
    (:`OnCompleted`
      (bind (_direction _alpha) (`Timeline|Timeline_1`)
        (:`Update`
          (`self.K2_SetActorRotation` (`KismetMathLibrary.RLerp` (`self.K2_GetActorRotation`) (`KismetMathLibrary.MakeRotator` _returnvalue_roll _returnvalue_pitch _returnvalue_yaw) _alpha)))
        (:`Finished`
          (`|PlayMontage` (`self.Mesh`) "/Game/Talking_Montage.Talking_Montage"
            (:`OnCompleted`
              (`|AIMoveTo` self (0.0 0.0 0.0) (`self.WeiStart`) 5.0 true))))))))

(event `/Game/Blueprints/NPC/WidgetNPCInteraction.ConversationOpening`)

(event `/Game/Blueprints/NPC/WidgetNPCInteraction.ReactToResponse`
  (params (Response :type Integer)))

(event `self.ReceiveBeginPlay`
  (`parent.ReceiveBeginPlay`)
  (if (not (`self.untalkable`))
    (set `/Game/Blueprints/NPC/WID_InteractionOptions.SpeificNpc` self (`self.TalkingWidget`))))

(event `WIEMOBILE`
  (`KismetSystemLibrary.Delay` 2.0)
  (bind _aswid_interaction_options (cast `/Game/Blueprints/NPC/WID_InteractionOptions` (`WidgetComponent.GetUserWidgetObject` (`self.TalkingOptions`))))
  (`/Game/Blueprints/NPC/WID_InteractionOptions.StartDialogue` _aswid_interaction_options))

(fn `CheckCondition`
  (params (ConditionName :type "Name (by ref)"))
  (returns (ReturnValue :type Boolean))
  (return false))

(fn `GetBoolValue`
  (params (ValueName :type "Name (by ref)"))
  (returns (ReturnValue :type Boolean))
  (return false))

(fn `GetFloatValue`
  (params (ValueName :type "Name (by ref)"))
  (returns (ReturnValue :type "Float (double-precision)"))
  (return 0.0))

(fn `GetIntValue`
  (params (ValueName :type "Name (by ref)"))
  (returns (ReturnValue :type Integer))
  (return 0))

(fn `GetNameValue`
  (params (ValueName :type "Name (by ref)"))
  (returns (ReturnValue :type Name))
  (return (`self.DLGName`)))

(fn `GetParticipantDisplayName`
  (params (ActiveSpeaker :type Name))
  (returns (ReturnValue :type Text))
  (return ""))

(fn `GetParticipantGender`
  (returns (ReturnValue :type "ETextGender Enum"))
  (return "Masculine"))

(fn `GetParticipantIcon`
  (params (ActiveSpeaker :type Name) (ActiveSpeakerState :type Name))
  (returns (ReturnValue :type "Texture2D Object Reference"))
  (return "/Game/Blueprints/NPC/UI/WEI.WEI"))

(fn `GetParticipantName`
  (returns (ReturnValue :type Name))
  (return (`self.DLGName`)))

(fn `InitiateDialogue`
  (bind _ascagney_controller (cast `/Game/FirstPersonBP/Blueprints/CagneyController` (`GameplayStatics.GetPlayerController` 0)))
  (`/Game/FirstPersonBP/Blueprints/CagneyController.StartDialogue` _ascagney_controller (`self.Dialogue`) self))

(fn `ModifyBoolValue`
  (params (ValueName :type "Name (by ref)") (bNewValue :type Boolean))
  (returns (ReturnValue :type Boolean))
  (return false))

(fn `ModifyFloatValue`
  (params (ValueName :type "Name (by ref)") (bDelta :type Boolean) (Value :type "Float (double-precision)"))
  (returns (ReturnValue :type Boolean))
  (return false))

(fn `ModifyIntValue`
  (params (ValueName :type "Name (by ref)") (bDelta :type Boolean) (Value :type Integer))
  (returns (ReturnValue :type Boolean))
  (return false))

(fn `ModifyNameValue`
  (params (ValueName :type "Name (by ref)") (NameValue :type "Name (by ref)"))
  (returns (ReturnValue :type Boolean))
  (return false))

(fn `OnDialogueEvent`
  (params (EventName :type "Name (by ref)"))
  (returns (ReturnValue :type Boolean))
  (`|SwitchDialogueCallbackEvent` EventName
    (:`FlipBug`
      (set `self.bug` false))
    (:`TriggerDatBoost`
      (`self.TriggerBoost`))))

(fn `UserConstructionScript`)