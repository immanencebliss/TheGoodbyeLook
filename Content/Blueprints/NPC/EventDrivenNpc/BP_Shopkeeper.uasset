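; Shopkeeper NPC that talks to the player as a dialogue-plugin participant and moves between scripted points.
; It registers with its talking widget unless untalkable, and InitiateDialogue starts its dialogue through CagneyController.
; GoUpstairs, GoDownstairs and StealthEvent use AI MoveTo toward stair or detection points, with GoDownstairs swapping in BandarDialogue on arrival.
; OnDialogueEvent forwards event names to SwitchDialogueCallbackEvent; condition and value callbacks are mostly stubs.
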(event `/Game/Blueprints/NPC/WidgetNPCInteraction.ConversationOpening`)

(event `/Game/Blueprints/NPC/WidgetNPCInteraction.ReactToResponse`
  (params (Response :type Integer)))

(event `self.ReceiveBeginPlay`
  (`parent.ReceiveBeginPlay`)
  (if (not (`self.untalkable`))
    (set `/Game/Blueprints/NPC/WID_InteractionOptions.SpeificNpc` self (`self.TalkingWidget`))))

(event `GoUpstairs`
  (`|AIMoveTo` self (0.0 0.0 0.0) (`self.Upstairs`) 1.0 true
    (:`OnSuccess`
      (`|AIMoveTo` self (0.0 0.0 0.0) (`self.DetectionPoint`) 1.0))
    (:`OnFail`
      (`KismetSystemLibrary.PrintString` "FAil" true true (struct :`R` 1.0 :`G` 0.063118 :`A` 1.0)))))

(event `Go Downstairs`
  (`|AIMoveTo` self (0.0 0.0 0.0) (`self.DonwStairs`) 1.0
    (:`OnSuccess`
      (set `self.Dialogue` "/Game/Dialogues/BandarDialogue.BandarDialogue"))
    (:`OnFail`
      (`KismetSystemLibrary.PrintString` "FAil" true true (struct :`R` 1.0 :`G` 0.063118 :`A` 1.0)))))

(event `StealthEvent`
  (`KismetSystemLibrary.Delay` 2.5)
  (`|AIMoveTo` self (0.0 0.0 0.0) (`self.DetectionPoint`) 1.0))

(fn `CheckCondition`
  (params (ConditionName :type "Name (by ref)"))
  (returns (ReturnValue :type Boolean))
  (return false))

(fn `GetBoolValue`
  (params (ValueName :type "Name (by ref)"))
  (returns (ReturnValue :type Boolean))
  (return false))

(fn `GetFloatValue`
  (params (ValueName :type "Name (by ref)"))
  (returns (ReturnValue :type "Float (double-precision)"))
  (return 0.0))

(fn `GetIntValue`
  (params (ValueName :type "Name (by ref)"))
  (returns (ReturnValue :type Integer))
  (return 0))

(fn `GetNameValue`
  (params (ValueName :type "Name (by ref)"))
  (returns (ReturnValue :type Name))
  (return (`self.DLGName`)))

(fn `GetParticipantDisplayName`
  (params (ActiveSpeaker :type Name))
  (returns (ReturnValue :type Text))
  (return ""))

(fn `GetParticipantGender`
  (returns (ReturnValue :type "ETextGender Enum"))
  (return "Masculine"))

(fn `GetParticipantIcon`
  (params (ActiveSpeaker :type Name) (ActiveSpeakerState :type Name))
  (returns (ReturnValue :type "Texture2D Object Reference"))
  (return "/Engine/EditorResources/Ai_Spawnpoint.Ai_Spawnpoint"))

(fn `GetParticipantName`
  (returns (ReturnValue :type Name))
  (return (`self.DLGName`)))

(fn `InitiateDialogue`
  (bind _ascagney_controller (cast `/Game/FirstPersonBP/Blueprints/CagneyController` (`GameplayStatics.GetPlayerController` 0)))
  (`/Game/FirstPersonBP/Blueprints/CagneyController.StartDialogue` _ascagney_controller (`self.Dialogue`) self))

(fn `ModifyBoolValue`
  (params (ValueName :type "Name (by ref)") (bNewValue :type Boolean))
  (returns (ReturnValue :type Boolean))
  (return false))

(fn `ModifyFloatValue`
  (params (ValueName :type "Name (by ref)") (bDelta :type Boolean) (Value :type "Float (double-precision)"))
  (returns (ReturnValue :type Boolean))
  (return false))

(fn `ModifyIntValue`
  (params (ValueName :type "Name (by ref)") (bDelta :type Boolean) (Value :type Integer))
  (returns (ReturnValue :type Boolean))
  (return false))

(fn `ModifyNameValue`
  (params (ValueName :type "Name (by ref)") (NameValue :type "Name (by ref)"))
  (returns (ReturnValue :type Boolean))
  (return false))

(fn `OnDialogueEvent`
  (params (EventName :type "Name (by ref)"))
  (returns (ReturnValue :type Boolean))
  (`|SwitchDialogueCallbackEvent` EventName))

(fn `UserConstructionScript`)