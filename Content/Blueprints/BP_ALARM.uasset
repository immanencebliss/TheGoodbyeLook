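; BP_ALARM is an alarm light actor that, when AlarmEvent fires, switches the lighting to spotlights and starts a rotating, audible warning.
; The event hides the referenced point lights, shows the spotlights, unpauses audio and brightens the container's dynamic material, created in the construction script.
; The LIGHTLOOP timeline spins the root through a full yaw turn and restarts itself on finish, looping indefinitely.
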(event `self.ReceiveBeginPlay`
  (set `self.StartingRotation` (`SceneComponent.K2_GetComponentRotation` (`self.DefaultSceneRoot`)))
  (`AudioComponent.SetPaused` (`self.Audio`) true))

(event `AlarmEvent`
  (bind _startingrotation (`self.StartingRotation`))
  (for _array_element (`self.PointLights`)
    (`SceneComponent.SetVisibility` (`PointLight.PointLightComponent` _array_element) false false))
  (for _array_element_2 (`self.Spotlights`)
    (`SceneComponent.SetVisibility` (`SpotLight.SpotLightComponent` _array_element_2) true false))
  (`AudioComponent.SetPaused` (`self.Audio`) false)
  (`MaterialInstanceDynamic.SetScalarParameterValue` (`self.Matieral`) "bright" 5.0)
  (bind (_direction _lightrotate) (`Timeline|LIGHTLOOP` :!label _label)
    (:`Update`
      (`SceneComponent.K2_SetWorldRotation` (`self.DefaultSceneRoot`) (`KismetMathLibrary.RLerp` _startingrotation (`KismetMathLibrary.MakeRotator` (.roll _startingrotation) (.pitch _startingrotation) (+ (.yaw _startingrotation) 360.0)) _lightrotate) false false))
    (:`Finished`
      (`self.FromTheStart`))))

(event `FromTheStart`
  (goto _label :!via `PlayFromStart`))

(fn `UserConstructionScript`
  (bind _returnvalue (`PrimitiveComponent.CreateDynamicMaterialInstance` (`self.Container`) 0 "/Game/Blueprints/MAT_ALARMCOntainer_Inst.MAT_ALARMCOntainer_Inst" "None"))
  (set `self.Matieral` _returnvalue))