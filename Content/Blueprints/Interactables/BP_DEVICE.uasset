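; BP_DEVICE is an interactable device pickup that sets off the alarm sequence when the player takes it.
; On Interact it flags the BP_Cagney player as having the device, triggers the first BP_ALARM, and resets the first BP_BUG and starts its dialogue.
; It then calls PrepareFlee on every BP_Wei, with its own DestroyActor call inside that loop body.
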(event `/Game/Blueprints/Interactables/BI_Interactable.Interact`
  (params (Instigator :type "Actor Object Reference"))
  (bind _asbp_cagney (cast `/Game/FirstPersonBP/Blueprints/BP_Cagney` (`GameplayStatics.GetPlayerCharacter` 0)))
  (set `/Game/FirstPersonBP/Blueprints/BP_Cagney.HasDevice` true _asbp_cagney)
  (bind _outactors (`GameplayStatics.GetAllActorsOfClass` "/Game/Blueprints/BP_ALARM.BP_ALARM_C"))
  (`/Game/Blueprints/BP_ALARM.AlarmEvent` (`|GetArrayItem` _outactors))
  (bind _outactors_2 (`GameplayStatics.GetAllActorsOfClass` "/Game/Blueprints/NPC/BP_BUG.BP_BUG_C"))
  (bind _output (`|GetArrayItem` _outactors_2))
  (`/Game/Blueprints/NPC/BP_BUG.RESETBUG` _output)
  (`/Game/Blueprints/NPC/BP_BUG.Bug Dialogue` _output)
  (bind _outactors_3 (`GameplayStatics.GetAllActorsOfClass` "/Game/Blueprints/NPC/EventDrivenNpc/BP_Wei.BP_Wei_C"))
  (for _array_element _outactors_3
    (`/Game/Blueprints/NPC/EventDrivenNpc/BP_Wei.Prepare Flee` _array_element)
    (`self.K2_DestroyActor`)))

(fn `UserConstructionScript`
  (`parent.UserConstructionScript`))