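; Door Blueprint that toggles open and closed on interaction, with optional bell sounds when flagged as a shop door.
; Interact and OPENCLOSEDOOR share one toggle that plays or reverses a timeline, lerping the mesh's world rotation between Closed and Arrow component rotations.
; A BP_Shopkeeper entering the trigger with Canopen set also toggles it, gated by a DoOnce with no reset shown.
; The end-overlap tag check leads to no action.
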(event `OPENCLOSEDOOR`
  (if (`self.IsOpen`) :!label _label
    (set `self.IsOpen` false)
    (if (`self.IsShopDoor`)
      (`GameplayStatics.PlaySound2D` "/Game/Door_Shop_Bell_close.Door_Shop_Bell_close" 1.0 1.0 0.0 null null)
      (bind (_direction _alpha) (`Timeline|Timeline_0` :!via `Reverse` :!label _label_2)
        (:`Update`
          (`SceneComponent.K2_SetWorldRotation` (`self.StaticMesh`) (`KismetMathLibrary.RLerp` (`SceneComponent.K2_GetComponentRotation` (`self.Closed`)) (`SceneComponent.K2_GetComponentRotation` (`self.Arrow`)) _alpha true) false false)))
      (else
        (goto _label_2 :!via `Reverse`)))
    (else
      (set `self.IsOpen` true)
      (if (`self.IsShopDoor`)
        (`GameplayStatics.PlaySound2D` "/Game/Door_Shop_Bell_Open.Door_Shop_Bell_Open" 1.0 1.0 0.0 null null)
        (goto _label_2)
        (else
          (goto _label_2))))))

(event `/Game/Blueprints/Interactables/BI_Interactable.Interact`
  (params (Instigator :type "Actor Object Reference"))
  (goto _label))

(event `self.Trigger.OnComponentBeginOverlap`
  (params (OverlappedComponent :type "PrimitiveComponent Object Reference") (OtherActor :type "Actor Object Reference") (OtherComp :type "PrimitiveComponent Object Reference") (OtherBodyIndex :type Integer) (bFromSweep :type Boolean) (SweepResult :type "HitResult Structure (by ref)"))
  (bind _asbp_shopkeeper (cast `/Game/Blueprints/NPC/EventDrivenNpc/BP_Shopkeeper` OtherActor))
  (if (`/Game/Blueprints/NPC/EventDrivenNpc/BP_Shopkeeper.Canopen` _asbp_shopkeeper)
    (`/Engine/EditorBlueprintResources/StandardMacros.DoOnce` false
      (:`Completed`
        (`self.OPENCLOSEDOOR`)))))

(event `self.Trigger.OnComponentEndOverlap`
  (params (OverlappedComponent :type "PrimitiveComponent Object Reference") (OtherActor :type "Actor Object Reference") (OtherComp :type "PrimitiveComponent Object Reference") (OtherBodyIndex :type Integer))
  (if (`self.ActorHasTag` OtherActor "open")
    _))

(fn `UserConstructionScript`)