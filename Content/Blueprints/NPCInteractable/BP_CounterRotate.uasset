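; BP_CounterRotate is a counter piece that swings open when an actor tagged "counter" enters its AITRIGGER volume.
; BeginPlay caches the root's world rotation, and the overlap calls OpenCounter, which plays a timeline that lerps the whole root 90 degrees in negative roll from that rotation.
; CloseCounter is an empty event, so nothing in this Blueprint closes the counter again.
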(event `self.ReceiveBeginPlay`
  (set `self.StartingRotation` (`SceneComponent.K2_GetComponentRotation` (`self.DefaultSceneRoot`))))

(event `OpenCounter`
  (bind _startingrotation (`self.StartingRotation`))
  (bind (_direction _opencounter) (`Timeline|CounterOPENCLOSE`)
    (:`Update`
      (`SceneComponent.K2_SetWorldRotation` (`self.DefaultSceneRoot`) (`KismetMathLibrary.RLerp` _startingrotation (`KismetMathLibrary.MakeRotator` (- (.roll _startingrotation) 90.0) (.pitch _startingrotation) (.yaw _startingrotation)) _opencounter) false false))))

(event `CloseCounter`)

(event `self.AITRIGGER.OnComponentBeginOverlap`
  (params (OverlappedComponent :type "PrimitiveComponent Object Reference") (OtherActor :type "Actor Object Reference") (OtherComp :type "PrimitiveComponent Object Reference") (OtherBodyIndex :type Integer) (bFromSweep :type Boolean) (SweepResult :type "HitResult Structure (by ref)"))
  (if (`self.ActorHasTag` OtherActor "counter")
    (`self.OpenCounter`)))

(fn `UserConstructionScript`)