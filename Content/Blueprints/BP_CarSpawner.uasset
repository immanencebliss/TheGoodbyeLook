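; Car spawner actor that repeatedly spawns random cars and gives each a point to drive to.
; BeginPlay starts a looping Spawn timer with a random interval, picked once per spawner.
; Spawn picks a class from Cars and places it at the root's location, with world yaw flipped by Rotate180.
; A switch on the array index casts to one of four car classes to set DriveTo, so Cars order must match.
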(event `self.ReceiveBeginPlay`
  (`KismetSystemLibrary.K2_SetTimer` self "Spawn" (`KismetMathLibrary.RandomFloatInRange` 1.0 5.0) true))

(fn `Spawn`
  (set `self.RandomcarNum` (`KismetMathLibrary.RandomIntegerInRange` 0 (- (`KismetArrayLibrary.Array_Length` (`self.Cars`)) 1)))
  (if (`self.Rotate180`)
    (set `self.CarRotation` 180.0)
    (else
      (set `self.CarRotation` 0.0)))
  (bind _returnvalue (`|SpawnActorFromClass` (`|GetArrayItem` (`self.Cars`) (`self.RandomcarNum`)) (`KismetMathLibrary.MakeTransform` (.location (`SceneComponent.K2_GetComponentToWorld` (`self.DefaultSceneRoot`))) (`KismetMathLibrary.MakeRotator` 0.0 0.0 (`self.CarRotation`))) "Undefined" "OverrideRootScale" null null))
  (switch `int` (`self.RandomcarNum`)
    (:`0`
      (bind _ascar (cast `/Game/Blueprints/Car` _returnvalue))
      (set `/Game/Blueprints/Car.DriveTo` (`self.DriveToPoint`) _ascar))
    (:`1`
      (bind _ascarnumero_2 (cast `/Game/Blueprints/Carnumero2` _returnvalue))
      (set `/Game/Blueprints/Carnumero2.DriveTo` (`self.DriveToPoint`) _ascarnumero_2))
    (:`2`
      (bind _ascarnumero_3 (cast `/Game/Blueprints/Carnumero3` _returnvalue))
      (set `/Game/Blueprints/Carnumero3.DriveTo` (`self.DriveToPoint`) _ascarnumero_3))
    (:`3`
      (bind _ascarnumero_4 (cast `/Game/Blueprints/Carnumero4` _returnvalue))
      (set `/Game/Blueprints/Carnumero4.DriveTo` (`self.DriveToPoint`) _ascarnumero_4))))

(fn `UserConstructionScript`)