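; BP_NPC is an NPC Blueprint with world-space widget components for a speech box and talking options.
; On BeginPlay it passes the SocialWidget's WID_SpeechBox to the TalkingOptions' WID_InteractionOptions, linking the options UI to the speech box.
; Every Tick it turns SocialWidget toward the BP_Cagney player's first-person camera, changing only yaw so the widget keeps its pitch and roll.
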(event `self.ReceiveBeginPlay`
  (set `/Game/Blueprints/WID_InteractionOptions.SpeechBox` (cast `/Game/Blueprints/WID_SpeechBox` (`WidgetComponent.GetUserWidgetObject` (`self.SocialWidget`)) :!pure true) (cast `/Game/Blueprints/WID_InteractionOptions` (`WidgetComponent.GetUserWidgetObject` (`self.TalkingOptions`)) :!pure true)))

(event `self.ReceiveTick`
  (params (DeltaSeconds :type "Float (single-precision)"))
  (bind _socialwidget (`self.SocialWidget`))
  (`SceneComponent.K2_SetWorldRotation` _socialwidget (`KismetMathLibrary.MakeRotator` (.roll (`SceneComponent.K2_GetComponentRotation` _socialwidget)) (.pitch (`SceneComponent.K2_GetComponentRotation` _socialwidget)) (.yaw (`KismetMathLibrary.FindLookAtRotation` (`SceneComponent.K2_GetComponentLocation` (`self.SocialWidget`)) (`SceneComponent.K2_GetComponentLocation` (`/Game/FirstPersonBP/Blueprints/BP_Cagney.FirstPersonCamera` (cast `/Game/FirstPersonBP/Blueprints/BP_Cagney` (`GameplayStatics.GetPlayerCharacter` 0) :!pure true)))))) false false))

(fn `UserConstructionScript`)