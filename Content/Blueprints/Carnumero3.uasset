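; Carnumero3 is an actor, apparently a car, that drives itself to a target actor and then disappears.
; On BeginPlay it stores the root component's location, then plays the Drive timeline to lerp the root toward DriveTo's X and Y, keeping the starting height.
; Movement runs without sweep and only while DriveTo is valid, and the actor destroys itself when the timeline finishes.
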(event `self.ReceiveBeginPlay`
  (bind _currentlocation (`self.CurrentLocation`))
  (bind _driveto (`self.DriveTo`))
  (set `self.CurrentLocation` (`SceneComponent.K2_GetComponentLocation` (`self.DefaultSceneRoot`)))
  (bind (_direction _drivetrack) (`Timeline|Drive` :!via `PlayFromStart`)
    (:`Update`
      (`/Engine/EditorBlueprintResources/StandardMacros.IsValid` _driveto
        (:`Is Valid`
          (`SceneComponent.K2_SetWorldLocation` (`self.DefaultSceneRoot`) (`KismetMathLibrary.VLerp` _currentlocation (`KismetMathLibrary.MakeVector` (.x (`self.K2_GetActorLocation` _driveto)) (.y (`self.K2_GetActorLocation` _driveto)) (.z _currentlocation)) _drivetrack) false false))))
    (:`Finished`
      (`self.K2_DestroyActor`))))

(fn `UserConstructionScript`)