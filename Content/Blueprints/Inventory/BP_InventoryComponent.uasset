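; Inventory component that holds items as slot structures in an array sized to a set slot count.
; On BeginPlay it resizes the array and refreshes preset slots from their item class defaults.
; Adding tops up a partial stack of the same class, recursing with any overflow, or fills an empty slot.
; Adds always return true, with no check for a full inventory.
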(event `self.ReceiveBeginPlay`
  (`self.PrepareInventory`))

(fn `AddToInventory`
  (params (ContentToAdd :type "/Game/Blueprints/Inventory/SlotStructure Structure"))
  (returns (Success :type Boolean))
  (if (`.IsStackable_14_2B6B3C874A78010C5BF94FA05B52034C` (break `/Game/Blueprints/Inventory/ItemStructure` (break `/Game/Blueprints/Inventory/SlotStructure` ContentToAdd)))
    (bind _slotindex (`self.HasPartialStack` (`local.ContentToAdd`))
      (:`True`
        (`self.AddToStack` (`local.ContentToAdd`) _slotindex)
        (`KismetSystemLibrary.PrintString` "AddedToStack"))
      (:`False`
        (`self.CreateStack` (`local.ContentToAdd`) :!label _label)
        (`KismetSystemLibrary.PrintString` "CreateStack")))
    (else
      (goto _label)))
  (return true))

(fn `AddToStack`
  (params (SlotStructure :type "/Game/Blueprints/Inventory/SlotStructure Structure") (SlotIndex :type Integer))
  (returns (Success :type Boolean))
  (locals (CurrentStackQuantity :type Integer))
  (bind _slotindex (`local.SlotIndex`))
  (bind (_slotstructure_itemstructure _slotstructure_quantity) (break `/Game/Blueprints/Inventory/SlotStructure` (`local.SlotStructure`)))
  (bind _inventory (`self.Inventory`))
  (bind _slotstructure_itemstructure_2 (break `/Game/Blueprints/Inventory/SlotStructure` (`local.SlotStructure`)))
  (bind (_slotstructure_itemstructure_3 _slotstructure_quantity_2) (break `/Game/Blueprints/Inventory/SlotStructure` (`local.SlotStructure`)))
  (bind (_name _isstackable _mesh _description _isconsumable _maxstacksize) (break `/Game/Blueprints/Inventory/ItemStructure` _slotstructure_itemstructure_2))
  (bind _output (`|GetArrayItem` (`self.Inventory`) SlotIndex))
  (bind (_output_itemstructure _output_quantity) (break `/Game/Blueprints/Inventory/SlotStructure` (`|GetArrayItem` _inventory _slotindex)))
  (bind _output_get (set `local.CurrentStackQuantity` (`.Quantity_5_BB697E464BAEC821C7E72CA7FD6254EB` (break `/Game/Blueprints/Inventory/SlotStructure` _output))))
  (if (> (+ _output_get (`.Quantity_5_BB697E464BAEC821C7E72CA7FD6254EB` (break `/Game/Blueprints/Inventory/SlotStructure` SlotStructure))) (`.MaxStackSize_20_D1F9BF3940A68B3F43682EAEB3A6250F` (break `/Game/Blueprints/Inventory/ItemStructure` (break `/Game/Blueprints/Inventory/SlotStructure` _output))))
    (`KismetArrayLibrary.Array_Set` (`self.Inventory`) (`local.SlotIndex`) (make `/Game/Blueprints/Inventory/SlotStructure` _slotstructure_itemstructure_2 _maxstacksize))
    (`self.AddToInventory` (make `/Game/Blueprints/Inventory/SlotStructure` _slotstructure_itemstructure_3 (- _slotstructure_quantity_2 (- _maxstacksize (`local.CurrentStackQuantity`)))))
    (else
      (`KismetArrayLibrary.Array_Set` _inventory _slotindex (make `/Game/Blueprints/Inventory/SlotStructure` _output_itemstructure (+ _output_quantity _slotstructure_quantity)))))
  (return true))

(fn `CreateStack`
  (params (ContentToAdd :type "/Game/Blueprints/Inventory/SlotStructure Structure"))
  (bind _inventory (`self.Inventory`))
  (`KismetArrayLibrary.Array_Set` _inventory (`KismetArrayLibrary.Array_Find` _inventory (make `/Game/Blueprints/Inventory/SlotStructure` (struct :`IsStackable` true :`IsConsumable` true :`MaxStackSize` 4))) ContentToAdd))

(fn `PrepareInventory`
  (`KismetArrayLibrary.Array_Resize` (`self.Inventory`) (`self.NumberOfSlots`))
  (for (_array_element _array_index) (`self.Inventory`)
    (bind (_name _isstackable _mesh _description _isconsumable _maxstacksize _price _class) (break `/Game/Blueprints/Inventory/ItemStructure` (break `/Game/Blueprints/Inventory/SlotStructure` _array_element)))
    (if (`KismetSystemLibrary.IsValidClass` _class)
      (`KismetArrayLibrary.Array_Set` (`self.Inventory`) _array_index (make `/Game/Blueprints/Inventory/SlotStructure` (defaults `/Game/Blueprints/Inventory/BP_InventoryComponent` _class) (`.Quantity_5_BB697E464BAEC821C7E72CA7FD6254EB` (break `/Game/Blueprints/Inventory/SlotStructure` _array_element)))))))