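; Enemy character Blueprint that supplies patrol destinations and wait times from a list of Food, Smoke and Phone Call tasks.
; GenerateRandomTaskArray fills the list randomly, rerolling to avoid consecutive repeats.
; GiveNextPatrolLocation maps each task to a BP_PatrolLocations actor and its wait time, then returns the fourth location once tasks run out, reusing the last wait.
; Event graph is empty, and construction-script mesh and sensing-radius debug logic are unconnected.
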(event `self.ReceiveBeginPlay`)

(fn `GenerateRandomTaskArray`
  (bind _tasks (`self.tasks`))
  (for _index (range (+ (`KismetArrayLibrary.Array_Length` (`self.tasks`)) 1))
    (set `self.randomNum` (`KismetMathLibrary.RandomInteger` 3) :!label _label)
    (if (== (`self.randomNum`) (`self.previousRandNum`))
      (goto _label)
      (else
        (switch `int` (`self.randomNum`)
          (:`0`
            (`KismetArrayLibrary.Array_Set` _tasks _index "NewEnumerator0")
            (set `self.previousRandNum` 0))
          (:`1`
            (`KismetArrayLibrary.Array_Set` _tasks _index "NewEnumerator1")
            (set `self.previousRandNum` 1))
          (:`2`
            (`KismetArrayLibrary.Array_Set` _tasks _index "NewEnumerator2")
            (set `self.previousRandNum` 2)))))))

(fn `GetLocationBasedOnTask`
  (params (EnumType :type "/Game/AI/ENU_PedestrianTask Enum" :default "NewEnumerator0"))
  (returns (locationIndex :type Integer))
  (switch `/Game/AI/ENU_PedestrianTask` EnumType
    (:`NewEnumerator0`
      (return 0))
    (:`NewEnumerator1`
      (return 1))
    (:`NewEnumerator2`
      (return 2))))

(fn `GiveNextPatrolLocation`
  (returns (CustomWait :type "Float (double-precision)") (NextLocation :type "Actor Object Reference"))
  (locals (SetWaitTime :type "Float (double-precision)" :default 0.0))
  (if (> (`self.Point In Patrol`) (- (`KismetArrayLibrary.Array_Length` (`self.tasks`)) 1))
    (bind _asbp_patrol_locations (cast `/Game/AI/BP_PatrolLocations` (`|GetArrayItem` (`self.Patrol Locations`) 3)))
    (return (`local.SetWaitTime`) _asbp_patrol_locations)
    (else
      (bind _locationindex (`self.GetLocationBasedOnTask` (`|GetArrayItem` (`self.tasks`) (`self.Point In Patrol`))))
      (bind _asbp_patrol_locations_2 (cast `/Game/AI/BP_PatrolLocations` (`|GetArrayItem` (`self.Patrol Locations`) _locationindex))
        (:`then`
          (set `local.SetWaitTime` (`/Game/AI/BP_PatrolLocations.Waittime` _asbp_patrol_locations_2)))
        (:`CastFailed`
          (set `local.SetWaitTime` 0.0)))
      (`/Engine/EditorBlueprintResources/StandardMacros.IncrementInt` (`self.Point In Patrol`)
        (:`  `
          (return (`local.SetWaitTime`) _asbp_patrol_locations_2))))))

(fn `UserConstructionScript`)