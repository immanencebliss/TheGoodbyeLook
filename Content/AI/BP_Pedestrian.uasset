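; Pedestrian AI Blueprint that supplies patrol destinations and wait times for a randomized routine of food, smoking and phone-call stops.
; GenerateRandomTaskArray builds a short, random-length task list, rerolling to avoid back-to-back repeats.
; GiveNextPatrolLocation steps through that list, resolving each task to a random placed location actor of the matching class, then returns a random home location once tasks run out.
; The event graph is empty, so nothing here calls these functions.
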(event `self.ReceiveBeginPlay`)

(fn `GenerateRandomTaskArray`
  (locals (CurrentSlot :type Integer))
  (bind _tasks (`self.tasks`))
  (for _index (range (+ (`KismetMathLibrary.RandomIntegerInRange` 1 5) 1))
    (set `local.CurrentSlot` _index)
    (`KismetArrayLibrary.Array_Add` (`self.tasks`) "NewEnumerator0")
    (set `self.randomNum` (`KismetMathLibrary.RandomInteger` 3) :!label _label)
    (if (== (`self.randomNum`) (`self.previousRandNum`))
      (goto _label)
      (else
        (switch `int` (`self.randomNum`)
          (:`0`
            (`KismetArrayLibrary.Array_Set` _tasks (`local.CurrentSlot`) "NewEnumerator0"))
          (:`1`
            (`KismetArrayLibrary.Array_Set` _tasks (`local.CurrentSlot`) "NewEnumerator1"))
          (:`2`
            (`KismetArrayLibrary.Array_Set` _tasks (`local.CurrentSlot`) "NewEnumerator2")))
        (set `self.previousRandNum` (`self.randomNum`))))))

(fn `GetHomeLocation`
  (returns (Waittime :type "Float (double-precision)") (`AsBP Location` :type "Actor Object Reference"))
  (bind _outactors (`GameplayStatics.GetAllActorsOfClass` "/Game/AI/LocationTypes/BP_HomeLocation.BP_HomeLocation_C"))
  (bind _output (`|GetArrayItem` _outactors (`KismetMathLibrary.RandomIntegerInRange` 0 (- (`KismetArrayLibrary.Array_Length` _outactors) 1))))
  (return (`/Game/AI/LocationTypes/BP_HomeLocation.Waittime` _output) _output))

(fn `GetLocationBasedOnTask`
  (params (EnumType :type "/Game/AI/ENU_PedestrianTask Enum" :default "NewEnumerator0"))
  (returns (Waittime :type "Float (double-precision)") (`AsBP Location` :type "Actor Object Reference"))
  (switch `/Game/AI/ENU_PedestrianTask` EnumType
    (:`NewEnumerator0`
      (bind _outactors (`GameplayStatics.GetAllActorsOfClass` "/Game/AI/LocationTypes/BP_FoodLocation.BP_FoodLocation_C"))
      (bind _output (`|GetArrayItem` _outactors (`KismetMathLibrary.RandomIntegerInRange` 0 (- (`KismetArrayLibrary.Array_Length` _outactors) 1))))
      (return (`/Game/AI/LocationTypes/BP_FoodLocation.Waittime` _output) _output))
    (:`NewEnumerator1`
      (bind _outactors_2 (`GameplayStatics.GetAllActorsOfClass` "/Game/AI/LocationTypes/BP_SmokingLocation.BP_SmokingLocation_C"))
      (bind _output_2 (`|GetArrayItem` _outactors_2 (`KismetMathLibrary.RandomIntegerInRange` 0 (- (`KismetArrayLibrary.Array_Length` _outactors_2) 1))))
      (return (`/Game/AI/LocationTypes/BP_SmokingLocation.Waittime` _output_2) _output_2))
    (:`NewEnumerator2`
      (bind _outactors_3 (`GameplayStatics.GetAllActorsOfClass` "/Game/AI/LocationTypes/BP_CallLocation.BP_CallLocation_C"))
      (bind _output_3 (`|GetArrayItem` _outactors_3 (`KismetMathLibrary.RandomIntegerInRange` 0 (- (`KismetArrayLibrary.Array_Length` _outactors_3) 1))))
      (return (`/Game/AI/LocationTypes/BP_CallLocation.Waittime` _output_3) _output_3))))

(fn `GiveNextPatrolLocation`
  (returns (CustomWait :type "Float (double-precision)") (NextLocation :type "Actor Object Reference"))
  (locals (SetWaitTime :type "Float (double-precision)" :default 0.0))
  (if (> (`self.Point In Patrol`) (- (`KismetArrayLibrary.Array_Length` (`self.tasks`)) 1))
    (bind (_waittime _asbp_location) (`self.GetHomeLocation`))
    (return _waittime _asbp_location)
    (else
      (bind (_waittime_2 _asbp_location_2) (`self.GetLocationBasedOnTask` (`|GetArrayItem` (`self.tasks`) (`self.Point In Patrol`))))
      (set `local.SetWaitTime` _waittime_2)
      (`/Engine/EditorBlueprintResources/StandardMacros.IncrementInt` (`self.Point In Patrol`)
        (:`  `
          (return (`local.SetWaitTime`) _asbp_location_2))))))

(fn `UserConstructionScript`)