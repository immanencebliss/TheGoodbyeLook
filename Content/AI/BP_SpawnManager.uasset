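; BP_SpawnManager populates the level with ambient AI pedestrians, spawning a random-sized batch at BeginPlay.
; Tick, throttled by a two-second Delay, counts existing pedestrians and spawns another batch unless they exceed AICapacity, so batches can overshoot it.
; Each pedestrian spawns with the ambient behavior tree at a random BP_SpawnLocations actor and gets a random skeletal mesh from SkeletalMeshes.
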(event `self.ReceiveBeginPlay`
  (`self.SpawnMultipleAI`))

(event `self.ReceiveTick`
  (params (DeltaSeconds :type "Float (single-precision)"))
  (`KismetSystemLibrary.Delay` 2.0)
  (bind _outactors (`GameplayStatics.GetAllActorsOfClass` "/Game/AI/BP_Pedestrian.BP_Pedestrian_C"))
  (if (not (> (- (`KismetArrayLibrary.Array_Length` _outactors) 1) (`self.AICapacity`)))
    (`self.SpawnMultipleAI`)))

(fn `GetSkeletalMesh`
  (returns (SkeletalMesh :type "SkeletalMesh Object Reference"))
  (bind _skeletalmeshes (`self.SkeletalMeshes`))
  (return (`|GetArrayItem` _skeletalmeshes (`KismetMathLibrary.RandomIntegerInRange` 0 (- (`KismetArrayLibrary.Array_Length` _skeletalmeshes) 1)))))

(fn `GetSpawnLocation`
  (returns (SpawnLocationTransform :type "Transform Structure"))
  (bind _outactors (`GameplayStatics.GetAllActorsOfClass` "/Game/AI/LocationTypes/BP_SpawnLocations.BP_SpawnLocations_C"))
  (return (`self.GetTransform` (`|GetArrayItem` _outactors (`KismetMathLibrary.RandomIntegerInRange` 0 (- (`KismetArrayLibrary.Array_Length` _outactors) 1))))))

(fn `SpawnAmbientAI`
  (bind _spawnlocationtransform (`self.GetSpawnLocation`))
  (bind _returnvalue (`AIBlueprintHelperLibrary.SpawnAIFromClass` "/Game/AI/BP_Pedestrian.BP_Pedestrian_C" "/Game/AI/BT_AmbientAIController.BT_AmbientAIController" (.location _spawnlocationtransform)))
  (bind _skeletalmesh (`self.GetSkeletalMesh`))
  (`SkinnedMeshComponent.SetSkinnedAssetAndUpdate` (`Character.Mesh` (cast `/Game/AI/BP_Pedestrian` _returnvalue :!pure true)) _skeletalmesh true))

(fn `SpawnMultipleAI`
  (for _ (range (+ (`KismetMathLibrary.RandomIntegerInRange` 0 (`self.MaxAINum`)) 1))
    (`self.SpawnAmbientAI`)))

(fn `UserConstructionScript`)