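; SingleDrawerBP is an interactive drawer prop that slides open or shut when the player presses E while looking at it.
; A box overlap enables and disables the actor's input, while the LookingatDrawer event sets the look flag.
; The OpenDrawer timeline drives the drawer's relative Y position and plays or reverses according to IsClosed.
; Tick derives IsClosed by checking whether the timeline value is zero.
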(event `Looking at Drawer`
  (params (`Is Looking At` :type Boolean))
  (set `self.Is Looking At` `Is Looking At`))

(event `Key|E`
  (params (Key :type "Key Structure"))
  (bind _returnvalue (`GameplayStatics.GetPlayerController` 0))
  (:`Pressed`
    (if (`self.Is Looking At`)
      (if (`self.Is Closed`)
        (bind (_direction _drawermovement) (`Timeline|Open Drawer` :!label _label)
          (:`Update`
            (`SceneComponent.K2_SetRelativeLocation` (`self.Drawer`) (`KismetMathLibrary.MakeVector` 0.0 _drawermovement) false false)
            (`self.DisableInput` _returnvalue)
            (`self.EnableInput` _returnvalue)))
        (else
          (goto _label :!via `Reverse`))))))

(event `self.ReceiveTick`
  (params (DeltaSeconds :type "Float (single-precision)"))
  (set `self.Is Closed` (== (stale `Key|E` _drawermovement) 0.0)))

(event `self.Box.OnComponentBeginOverlap`
  (params (OverlappedComponent :type "PrimitiveComponent Object Reference") (OtherActor :type "Actor Object Reference") (OtherComp :type "PrimitiveComponent Object Reference") (OtherBodyIndex :type Integer) (bFromSweep :type Boolean) (SweepResult :type "HitResult Structure (by ref)"))
  (`self.EnableInput` (`GameplayStatics.GetPlayerController` 0)))

(event `self.Box.OnComponentEndOverlap`
  (params (OverlappedComponent :type "PrimitiveComponent Object Reference") (OtherActor :type "Actor Object Reference") (OtherComp :type "PrimitiveComponent Object Reference") (OtherBodyIndex :type Integer))
  (`self.DisableInput` (`GameplayStatics.GetPlayerController` 0)))

(fn `UserConstructionScript`)