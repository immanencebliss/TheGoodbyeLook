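; Wall cabinet prop whose door swings on interaction.
; OnInteract plays or reverses the DoorMovement timeline based on IsClosed, and the timeline's update sets the door's relative yaw.
; Tick derives IsClosed every frame from whether the timeline value is at or below a fixed angle threshold.
; Each timeline update also disables and immediately re-enables the actor's input for the first player controller.
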(event `/Game/AFPC/Blueprints/AFPCharacter/Character/InteractInterface.OnInteract`
  (bind _returnvalue (`GameplayStatics.GetPlayerController` 0))
  (if (`self.Is Closed`)
    (`|ExecutionSequence`
      (:`then_1`
        (bind (_direction _door_movement) (`Timeline|Door Movement` :!label _label)
          (:`Update`
            (`SceneComponent.K2_SetRelativeRotation` (`self.Door`) (`KismetMathLibrary.MakeRotator` 0.0 0.0 _door_movement) false false)
            (`self.DisableInput` _returnvalue)
            (`self.EnableInput` _returnvalue)))))
    (else
      (`|ExecutionSequence`
        (:`then_0`
          (goto _label :!via `Reverse`))))))

(event `self.ReceiveTick`
  (params (DeltaSeconds :type "Float (single-precision)"))
  (set `self.Is Closed` (<= (stale `/Game/AFPC/Blueprints/AFPCharacter/Character/InteractInterface.OnInteract` _door_movement) -130.0)))

(fn `UserConstructionScript`)